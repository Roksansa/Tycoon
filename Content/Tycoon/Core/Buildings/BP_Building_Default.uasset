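; BP_Building_Default is a tycoon building that shows its placement and income state through the material on its apartment door corner mesh.
; On BeginPlay it binds to the placeable-switch and deposit-available events.
; Placement changes swap the first material slot between placeable and not-placeable materials.
; Deposit changes for this actor swap the same slot between the collect and placeable materials.
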(event `self.ReceiveBeginPlay`
  (add `self.OnSwitchPlaceable` (delegate `OnSwitchPlaceableMaterial`))
  (add `TPlaceableActor.OnChangeDepositAvailable` (delegate `OnChangeCollectIncomeEvent`)))

(event `OnSwitchPlaceableMaterial` :!signature `self.OnSwitchPlaceable`
  (params (bIsPlaceable :type Boolean))
  (`PrimitiveComponent.SetMaterial` (`self.SM_Bld_Apartment_Door_Corner_02`) 0 (select `bool` bIsPlaceable :`false` (`self.NotPlaceableMaterial`) :`true` (`self.PlaceableMaterial`) :!type "MaterialInterface Object Reference")))

(event `OnChangeCollectIncomeEvent`
  (params (Actor :type "TPlaceableActor Object Reference") (bDepositAvailable :type Boolean))
  (if (== Actor self)
    (`PrimitiveComponent.SetMaterial` (`self.SM_Bld_Apartment_Door_Corner_02`) 0 (select `bool` bDepositAvailable :`false` (`self.PlaceableMaterial`) :`true` (`self.CollectPlaceableMaterial`) :!type "MaterialInterface Object Reference"))))

(fn `UserConstructionScript`)