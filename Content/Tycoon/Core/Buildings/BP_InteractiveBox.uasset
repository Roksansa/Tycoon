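; BP_InteractiveBox is a clickable cube actor in the Tycoon buildings folder that changes color in response to the mouse.
; On BeginPlay it binds its click and end-cursor-over events and sets the cube's material to purple.
; A click sets a Clicked flag and turns the cube green.
; When the cursor leaves a clicked box, the flag clears and purple returns after a short delay.
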(event `EndMouseOverlap`
  (params (TouchedActor :type "Actor Object Reference"))
  (bind _cube (`self.Cube`))
  ;[1 1 1] End Mouse Overlay event
  (if (`self.Clicked`)
    (set `self.Clicked` false)
    (`KismetSystemLibrary.Delay` 0.2)
    (`/Engine/EditorBlueprintResources/StandardMacros.IsValid` _cube
      (:`Is Valid`
        (`PrimitiveComponent.SetMaterial` _cube 0 "/Game/Tycoon/Core/Buildings/MI_BaseColor_Purple.MI_BaseColor_Purple")))))

(event `self.ReceiveBeginPlay`
  (bind _cube (`self.Cube`))
  (add `Actor.OnClicked` (delegate `OnMouseClicked`))
  (add `Actor.OnEndCursorOver` (delegate `EndMouseOverlap`))
  ;[1 1 1] Set default material
  (`/Engine/EditorBlueprintResources/StandardMacros.IsValid` _cube
    (:`Is Valid`
      (`PrimitiveComponent.SetMaterial` _cube 0 "/Game/Tycoon/Core/Buildings/MI_BaseColor_Purple.MI_BaseColor_Purple"))))

(event `OnMouseClicked`
  (params (TouchedActor :type "Actor Object Reference") (ButtonPressed :type "Key Structure" :default "None"))
  (bind _cube (`self.Cube`))
  ;[1 1 1] On mouse clicked event
  (set `self.Clicked` true)
  (`/Engine/EditorBlueprintResources/StandardMacros.IsValid` _cube
    (:`Is Valid`
      (`PrimitiveComponent.SetMaterial` _cube 0 "/Game/Tycoon/Core/Buildings/MI_BaseColor_Green.MI_BaseColor_Green"))))

(fn `UserConstructionScript`)